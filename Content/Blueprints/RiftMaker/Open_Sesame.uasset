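; Open_Sesame is a collectible Rift Maker pickup that spins continuously around its yaw axis.
; When a BP_PlayerRig overlaps its mesh, a PickedUp flag blocks repeat collection and GM_State is told to add a rift maker.
; The actor is not destroyed: it hides the mesh, zeroes the Niagara spawn rate and plays a pitched-up gravity-change sound.
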(event `self.ReceiveTick`
  (params (DeltaSeconds :type "Float (single-precision)"))
  (`SceneComponent.K2_AddRelativeRotation` (`self.SM_RiftMaker`) (`KismetMathLibrary.MakeRotator` 0.0 0.0 (* DeltaSeconds 180.0)) false false))

(event `self.SM_RiftMaker.OnComponentBeginOverlap`
  (params (OverlappedComponent :type "PrimitiveComponent Object Reference") (OtherActor :type "Actor Object Reference") (OtherComp :type "PrimitiveComponent Object Reference") (OtherBodyIndex :type Integer) (bFromSweep :type Boolean) (SweepResult :type "HitResult Structure (by ref)"))
  (if (not (`self.PickedUp`))
    (bind _asbp_player_rig (cast `/Game/Blueprints/Player/Rig/BP_PlayerRig` OtherActor))
    (`/Engine/EditorBlueprintResources/StandardMacros.IsValid` _asbp_player_rig
      (:`Is Valid`
        (set `self.PickedUp` true)
        (bind _asgm_state (cast `/Game/Blueprints/GameModes/GM_State` (`GameplayStatics.GetGameState`)))
        (`/Engine/EditorBlueprintResources/StandardMacros.IsValid` _asgm_state
          (:`Is Valid`
            (`/Game/Blueprints/GameModes/GM_State.Add Rift Maker` _asgm_state)
            (`SceneComponent.SetVisibility` (`self.SM_RiftMaker`) false false)
            (`FXSystemComponent.SetFloatParameter` (`self.NS_RiftMaker`) "SpawnRate" 0.0)
            (`FXSystemComponent.SetFloatParameter` (`self.NS_RiftMaker`) "SpawnRate" 0.0)
            (`GameplayStatics.PlaySound2D` "/Game/Audio/Gravity/A_GravityChange.A_GravityChange" 1.0 1.5 0.0 null null)))))))

(fn `UserConstructionScript`)