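; Old player rig Blueprint: a physics-driven capsule character that moves, looks and jumps under an arbitrary gravity vector.
; Tick applies gravity as impulses, flags jumping when JumpDetector overlaps nothing, and eases Meshes toward capsule rotation.
; UpdateGravityVector realigns the capsule via GravCalc and WorldRot, briefly releasing its SixDOF constraint, as does yaw look.
; Enhanced Input drives impulse movement with grounded speed capping, jumps and clamped camera pitch.
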(event `self.ReceiveBeginPlay`
  (bind _returnvalue (pcsubsystem `EnhancedInputLocalPlayerSubsystem` (`GameplayStatics.GetPlayerController` 0)))
  (`/Engine/EditorBlueprintResources/StandardMacros.IsValid` _returnvalue
    (:`Is Valid`
      (`EnhancedInputSubsystemInterface.AddMappingContext` _returnvalue "/Game/Inputs/IMC_Player.IMC_Player" 0 (struct)))))

(event `UpdateGravityVector`
  (bind _capsulecomponent (`self.CapsuleComponent`))
  (`SceneComponent.K2_SetWorldRotation` (`self.GravCalc`) (`KismetMathLibrary.MakeRotator` 0.0 (.pitch (`KismetMathLibrary.Conv_VectorToRotator` (`KismetMathLibrary.Normal` (`self.GravityVector`)))) (.yaw (`KismetMathLibrary.Conv_VectorToRotator` (`KismetMathLibrary.Normal` (`self.GravityVector`))))) false false)
  (set `self.NewTargetWorldRot` (`SceneComponent.K2_GetComponentRotation` (`self.WorldRot`)))
  (bind _output_get (set `self.OldMeshWorldRot` (`SceneComponent.K2_GetComponentRotation` (`self.Meshes`))))
  (`PrimitiveComponent.SetConstraintMode` _capsulecomponent "None")
  (`SceneComponent.K2_SetWorldRotation` (`self.CapsuleComponent`) (`self.NewTargetWorldRot`) false false)
  (`SceneComponent.K2_SetWorldRotation` (`self.Meshes`) _output_get false false)
  (`PrimitiveComponent.SetConstraintMode` _capsulecomponent "SixDOF"))

(event `self.ReceiveTick`
  (params (DeltaSeconds :type "Float (single-precision)"))
  (`SceneComponent.K2_SetWorldRotation` (`self.Meshes`) (`KismetMathLibrary.RLerp` (`SceneComponent.K2_GetComponentRotation` (`self.Meshes`)) (`SceneComponent.K2_GetComponentRotation` (`self.CapsuleComponent`)) (* DeltaSeconds 8.0) true) false false)
  (`PrimitiveComponent.AddImpulse` (`self.CapsuleComponent`) (* (`self.GravityVector`) (`self.GravityStrength`)) "None" true)
  (set `self.IsJumping` (< (`KismetArrayLibrary.Array_Length` (`PrimitiveComponent.GetOverlappingActors` (`self.JumpDetector`) null)) 1)))

(event `self.ReceiveAsyncPhysicsTick`
  (params (DeltaSeconds :type "Float (single-precision)") (SimSeconds :type "Float (single-precision)")))

(event `EnhancedInput|/Game/Inputs/InputActions/Player/IA_Jump`
  (params (ActionValue :type Boolean) (ElapsedSeconds :type "Float (double-precision)") (TriggeredSeconds :type "Float (double-precision)") (InputAction :type "InputAction Object Reference" :default "/Game/Inputs/InputActions/Player/IA_Jump.IA_Jump"))
  (bind _returnvalue (* (`KismetMathLibrary.NegateVector` (`self.GravityVector`)) (`CharacterMovementComponent.JumpZVelocity` (`self.CharacterMovement`))))
  (:`Triggered`
    (`KismetSystemLibrary.PrintString` (`KismetStringLibrary.Conv_VectorToString` _returnvalue))
    (if (not (`self.IsJumping`))
      (`PrimitiveComponent.AddImpulse` (`self.CapsuleComponent`) _returnvalue "None" true)
      (`KismetSystemLibrary.PrintString` "WEEEEEEEEEEEEEEEEEEEEEEEEEEEEEEEEEEEEEEEEEEEEEEEEEEEEEEEEEEEEEEEEEEEEEEEEEEEEEEEEEEEEEEEEEEEEEEEEEEEEEEEEEEEEEEEE"))))

(event `EnhancedInput|/Game/Inputs/InputActions/Player/IA_Move`
  (params (ActionValue :type "Vector2D Structure") (ElapsedSeconds :type "Float (double-precision)") (TriggeredSeconds :type "Float (double-precision)") (InputAction :type "InputAction Object Reference" :default "/Game/Inputs/InputActions/Player/IA_Move.IA_Move"))
  (bind _capsulecomponent (`self.CapsuleComponent`))
  (bind _currentspeed (`self.CurrentSpeed`))
  (bind _maxspeed (`self.MaxSpeed`))
  (bind _returnvalue (`SceneComponent.GetComponentVelocity` _capsulecomponent))
  (bind _returnvalue_2 (`KismetMathLibrary.VSize` _returnvalue))
  (bind _returnvalue_3 (* _returnvalue (`SceneComponent.GetUpVector` _capsulecomponent)))
  (bind _returnvalue_4 (+ (* (`SceneComponent.GetForwardVector` _capsulecomponent) ActionValue_X) (* (`SceneComponent.GetRightVector` _capsulecomponent) ActionValue_Y)))
  (:`Triggered`
    (if (`self.IsJumping`)
      (`PrimitiveComponent.AddImpulse` _capsulecomponent (* _returnvalue_4 (`self.SpeedAir`)) "None" true)
      (else
        (if (< _currentspeed (`self.MaxSpeed`))
          _
          (else
            _))
        (`PrimitiveComponent.AddImpulse` _capsulecomponent (* _returnvalue_4 (`self.SpeedGround`)) "None" true)))
    (`KismetSystemLibrary.PrintString` (`KismetStringLibrary.Conv_DoubleToString` _currentspeed))
    (if (and (> _returnvalue_2 _maxspeed) (not (`self.IsJumping`)))
      (`PrimitiveComponent.SetPhysicsLinearVelocity` _capsulecomponent (+ (* (- _returnvalue _returnvalue_3) (/ _maxspeed _returnvalue_2)) _returnvalue_3) false "None"))
    (set `self.CurrentSpeed` _returnvalue_2)))

(event `EnhancedInput|/Game/Inputs/InputActions/Player/IA_Look`
  (params (ActionValue :type "Vector2D Structure") (ElapsedSeconds :type "Float (double-precision)") (TriggeredSeconds :type "Float (double-precision)") (InputAction :type "InputAction Object Reference" :default "/Game/Inputs/InputActions/Player/IA_Look.IA_Look"))
  (bind _capsulecomponent (`self.CapsuleComponent`))
  (bind _camrot (`self.CamRot`))
  (:`Triggered`
    (`PrimitiveComponent.SetConstraintMode` _capsulecomponent "None")
    (`SceneComponent.K2_AddLocalRotation` _capsulecomponent (`KismetMathLibrary.MakeRotator` 0.0 0.0 ActionValue_X) false false)
    (`PrimitiveComponent.SetConstraintMode` _capsulecomponent "SixDOF")
    (`SceneComponent.K2_SetRelativeRotation` _camrot (`KismetMathLibrary.MakeRotator` 0.0 (`KismetMathLibrary.FClamp` (+ (.pitch (`SceneComponent.RelativeRotation` _camrot)) ActionValue_Y) -80.0 80.0)) false false)))

(event `self.JumpDetector.OnComponentBeginOverlap`
  (params (OverlappedComponent :type "PrimitiveComponent Object Reference") (OtherActor :type "Actor Object Reference") (OtherComp :type "PrimitiveComponent Object Reference") (OtherBodyIndex :type Integer) (bFromSweep :type Boolean) (SweepResult :type "HitResult Structure (by ref)"))
  (`KismetSystemLibrary.PrintString` (`KismetStringLibrary.Conv_IntToString` (`KismetArrayLibrary.Array_Length` (`PrimitiveComponent.GetOverlappingActors` (`self.JumpDetector`) null))) :!label _label))

(event `self.JumpDetector.OnComponentEndOverlap`
  (params (OverlappedComponent :type "PrimitiveComponent Object Reference") (OtherActor :type "Actor Object Reference") (OtherComp :type "PrimitiveComponent Object Reference") (OtherBodyIndex :type Integer))
  (goto _label))

(fn `UserConstructionScript`)