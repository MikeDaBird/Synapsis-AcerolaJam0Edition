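; Physics-driven first-person player pawn with switchable gravity that carries and throws cubes and spends rift makers to open anomalies.
; Impulses on the capsule drive gravity, movement and jumping; gravity changes reorient it via a 360-step yaw search for the closest previous facing, while meshes lerp after it.
; Tick traces from the camera to feed grab and crosshair UI, holds cubes at PickupPoint, and updates the speedrun timer.
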(event `self.ReceiveBeginPlay`
  (bind _returnvalue (pcsubsystem `EnhancedInputLocalPlayerSubsystem` (`GameplayStatics.GetPlayerController` 0)))
  (`/Engine/EditorBlueprintResources/StandardMacros.IsValid` _returnvalue
    (:`Is Valid`
      (`EnhancedInputSubsystemInterface.AddMappingContext` _returnvalue "/Game/Inputs/IMC_Player.IMC_Player" 0 (struct))
      (bind _asgm_state (cast `/Game/Blueprints/GameModes/GM_State` (`GameplayStatics.GetGameState`)))
      (`/Engine/EditorBlueprintResources/StandardMacros.IsValid` _asgm_state
        (:`Is Valid`
          (set `self.GameState` _asgm_state)
          (bind _returnvalue_2 (`|CreateWidget` "/Game/Widgets/W_InGameUI.W_InGameUI_C" (`GameplayStatics.GetPlayerController` 0)))
          (bind _output_get (set `self.UIWidget` _returnvalue_2))
          (`UserWidget.AddToViewport` _output_get 0)
          (`KismetSystemLibrary.DelayUntilNextTick`)
          (`/Game/Blueprints/GameModes/GI_GameManager.Run Speedrun Timer` (`/Game/Blueprints/GameModes/GM_State.Game Instance` (`self.GameState`))))))))

(event `UpdateGravityVector`
  (bind _capsulecollider (`self.CapsuleCollider`))
  (bind _returnvalue (`SceneComponent.K2_GetComponentLocation` _capsulecollider))
  (bind _returnvalue_2 (`SceneComponent.GetUpVector` _capsulecollider))
  (bind _returnvalue_3 (`CapsuleComponent.GetScaledCapsuleHalfHeight` _capsulecollider))
  (`GameplayStatics.SpawnSound2D` "/Game/Audio/Gravity/A_GravityChange.A_GravityChange" 0.75 1.0 0.0 null true)
  (`SceneComponent.K2_SetWorldRotation` (`self.GravCalc`) (`KismetMathLibrary.MakeRotator` 0.0 (.pitch (`KismetMathLibrary.Conv_VectorToRotator` (`KismetMathLibrary.Normal` (`self.GravityVector`)))) (.yaw (`KismetMathLibrary.Conv_VectorToRotator` (`KismetMathLibrary.Normal` (`self.GravityVector`))))) false false)
  (set `self.OldPlayerRotation` (`SceneComponent.K2_GetComponentRotation` (`self.CapsuleCollider`)))
  (set `self.NewTargetWorldRot` (`SceneComponent.K2_GetComponentRotation` (`self.WorldRot`)))
  (bind _output_get (set `self.OldMeshWorldRot` (`SceneComponent.K2_GetComponentRotation` (`self.Meshes`))))
  (bind _new_rotation (`self.ReorientPlayerAfterGravitySwitch`))
  (`PrimitiveComponent.SetConstraintMode` _capsulecollider "None")
  (`SceneComponent.K2_SetWorldRotation` _capsulecollider _new_rotation false false)
  (`SceneComponent.K2_SetWorldRotation` (`self.Meshes`) _output_get false false)
  (`PrimitiveComponent.SetConstraintMode` _capsulecollider "SixDOF")
  (bind (_outhit _returnvalue_4) (`KismetSystemLibrary.LineTraceSingleForObjects` _returnvalue (+ _returnvalue (* (`KismetMathLibrary.NegateVector` _returnvalue_2) _returnvalue_3)) (`|MakeArray` "ObjectTypeQuery2" :!type "EObjectTypeQuery Enum")))
  (if _returnvalue_4
    (bind (_bblockinghit _binitialoverlap _time _distance) (`GameplayStatics.BreakHitResult` _outhit))
    (if (< _distance _returnvalue_3)
      (`SceneComponent.K2_SetWorldLocation` _capsulecollider (+ (* (* _returnvalue_2 (- _returnvalue_3 _distance)) (2.0 2.0 2.0)) (`SceneComponent.K2_GetComponentLocation` _capsulecollider)) false true))))

(event `self.ReceiveTick`
  (params (DeltaSeconds :type "Float (single-precision)"))
  (bind _pickuppoint (`self.PickupPoint`))
  (bind _camera (`self.Camera`))
  (bind _landingtrigger (`self.LandingTrigger`))
  (bind _isjumping (`self.IsJumping`))
  (bind _gamestate (`self.GameState`))
  (bind _returnvalue (`SceneComponent.K2_GetComponentLocation` _camera))
  (bind _returnvalue_2 (`SceneComponent.K2_GetComponentLocation` _pickuppoint))
  (bind _sm_cube (`/Game/Blueprints/Cube/BP_Cube.SM_Cube` (`self.HeldObject`)))
  (`SceneComponent.K2_SetWorldRotation` (`self.Meshes`) (`KismetMathLibrary.RLerp` (`SceneComponent.K2_GetComponentRotation` (`self.Meshes`)) (`SceneComponent.K2_GetComponentRotation` (`self.CapsuleCollider`)) (* DeltaSeconds 8.0) true) false false)
  (`PrimitiveComponent.AddImpulse` (`self.CapsuleCollider`) (* (`self.GravityVector`) (* (`self.GravityStrength`) (* DeltaSeconds 8000.0) (`self.CustomTimeDilation`))) "None" false)
  (`PrimitiveComponent.AddImpulse` (`self.CapsuleCollider`) (* (`self.GravityVector`) (* (`self.GravityStrength`) (* DeltaSeconds 8000.0) (`self.CustomTimeDilation`))) "None" false)
  (set `self.IsJumping` (< (`KismetArrayLibrary.Array_Length` (`PrimitiveComponent.GetOverlappingActors` (`self.JumpDetector`) null)) 1))
  (if (== (`self.IsHoldingState`) 2)
    (`SceneComponent.K2_SetWorldTransform` _sm_cube (`KismetMathLibrary.MakeTransform` _returnvalue_2 (`KismetMathLibrary.MakeRotFromX` (`SceneComponent.GetForwardVector` _pickuppoint))) true false)
    (`PrimitiveComponent.SetPhysicsLinearVelocity` _sm_cube (0.0 0.0 0.0) false "None")
    (`PrimitiveComponent.SetPhysicsAngularVelocityInDegrees` _sm_cube (0.0 0.0 0.0) false "None")
    (if (> (`KismetMathLibrary.Vector_Distance` _returnvalue_2 (`SceneComponent.K2_GetComponentLocation` _sm_cube)) 120.0)
      (`self.Release`))
    (else
      (set `self.CrosshairPointTest` false)
      (bind (_outhit _returnvalue_3) (`KismetSystemLibrary.LineTraceSingleForObjects` _returnvalue (+ (* (`SceneComponent.GetForwardVector` _camera) (`self.GrabDistance`)) _returnvalue) (`|MakeArray` "ObjectTypeQuery1" "ObjectTypeQuery2" "ObjectTypeQuery6" "ObjectTypeQuery5" "ObjectTypeQuery4" :!type "EObjectTypeQuery Enum")))
      (if _returnvalue_3
        (bind (_bblockinghit _binitialoverlap _time _distance _location _impactpoint _normal _impactnormal _physmat _hitactor) (`GameplayStatics.BreakHitResult` _outhit))
        (bind _asbp_cube (cast `/Game/Blueprints/Cube/BP_Cube` _hitactor)
          (:`then`
            (`/Engine/EditorBlueprintResources/StandardMacros.IsValid` _asbp_cube
              (:`Is Valid`
                (set `self.PointedObject` _asbp_cube)
                (set `self.CrosshairPointTest` true))
              (:`Is Not Valid`
                (set `self.PointedObject` null :!label _label)
                (bind _asbp_anomaly (cast `/Game/Blueprints/Anomalies/BP_Anomaly` _hitactor)
                  (:`then`
                    (`/Engine/EditorBlueprintResources/StandardMacros.IsValid` _asbp_anomaly
                      (:`Is Valid`
                        (set `self.PointedAnomaly` _asbp_anomaly)
                        (if (> (`/Game/Blueprints/GameModes/GM_State.AmountOfRiftMakers` (`self.GameState`)) 0)
                          (set `self.CrosshairPointTest` true)))
                      (:`Is Not Valid`
                        (set `self.PointedAnomaly` null :!label _label_2))))
                  (:`CastFailed`
                    (goto _label_2))))))
          (:`CastFailed`
            (goto _label)))
        (else
          (goto _label)))))
  (if (`self.CrosshairPointTest`)
    (`self.Point UI`)
    (else
      (`self.Unpoint UI`)))
  (if (!= _isjumping _landingtrigger)
    (set `self.LandingTrigger` _isjumping)
    (if (and (not _landingtrigger) (> (`GameplayStatics.GetTimeSeconds`) 0.5))
      (`GameplayStatics.PlaySound2D` "/Game/Audio/Footstep/A_Footstep_JumpLand_1.A_Footstep_JumpLand_1" 1.0 1.0 0.0 null null)))
  (`KismetSystemLibrary.DelayUntilNextTick`)
  (`/Engine/EditorBlueprintResources/StandardMacros.IsValid` _gamestate
    (:`Is Valid`
      (if (not (`/Game/Blueprints/GameModes/GM_State.IsDed` _gamestate))
        (`/Game/Blueprints/GameModes/GI_GameManager.Update Speedrun Timer` (`/Game/Blueprints/GameModes/GM_State.Game Instance` _gamestate))))))

(event `EnhancedInput|/Game/Inputs/InputActions/Player/IA_Jump`
  (params (ActionValue :type Boolean) (ElapsedSeconds :type "Float (double-precision)") (TriggeredSeconds :type "Float (double-precision)") (InputAction :type "InputAction Object Reference" :default "/Game/Inputs/InputActions/Player/IA_Jump.IA_Jump"))
  (:`Triggered`
    (if (not (`self.IsJumping`))
      (`PrimitiveComponent.AddImpulse` (`self.CapsuleCollider`) (* (* (`KismetMathLibrary.NegateVector` (`self.GravityVector`)) (`self.JumpStrength`)) (* (`GameplayStatics.GetWorldDeltaSeconds`) 100.0 (/ (`self.CustomTimeDilation`) (`GameplayStatics.GetGlobalTimeDilation`)))) "None" false)
      (set `self.AnimJump` true)
      (`KismetSystemLibrary.Delay` 0.1)
      (set `self.AnimJump` false))))

(event `EnhancedInput|/Game/Inputs/InputActions/Player/IA_Move`
  (params (ActionValue :type "Vector2D Structure") (ElapsedSeconds :type "Float (double-precision)") (TriggeredSeconds :type "Float (double-precision)") (InputAction :type "InputAction Object Reference" :default "/Game/Inputs/InputActions/Player/IA_Move.IA_Move"))
  (bind _capsulecollider (`self.CapsuleCollider`))
  (bind _returnvalue (`SceneComponent.GetComponentVelocity` _capsulecollider))
  (bind _returnvalue_2 (* (`self.MaxSpeed`) (`self.CustomTimeDilation`)))
  (bind _returnvalue_3 (`KismetMathLibrary.VSize` _returnvalue))
  (bind _returnvalue_4 (* (`KismetMathLibrary.Vector_GetAbs` _returnvalue) (`SceneComponent.GetUpVector` _capsulecollider)))
  (bind _returnvalue_5 (* (+ (* (`SceneComponent.GetForwardVector` _capsulecollider) ActionValue_X) (* (`SceneComponent.GetRightVector` _capsulecollider) ActionValue_Y)) (* (`GameplayStatics.GetWorldDeltaSeconds`) 10000.0 (/ (`self.CustomTimeDilation`) (`GameplayStatics.GetGlobalTimeDilation`)))))
  (:`Triggered`
    (if (`self.IsJumping`) :!label _label_3
      (`PrimitiveComponent.AddImpulse` _capsulecollider (* _returnvalue_5 (`self.SpeedAir`)) "None" false)
      (else
        (if (< (`self.CurrentSpeed`) (`self.MaxSpeed`))
          _
          (else
            _))
        (`PrimitiveComponent.AddImpulse` _capsulecollider (* _returnvalue_5 (`self.SpeedGround`)) "None" false)))
    (if (and (> _returnvalue_3 _returnvalue_2) (not (`self.IsJumping`)))
      (`PrimitiveComponent.SetPhysicsLinearVelocity` _capsulecollider (+ (* (- _returnvalue _returnvalue_4) (/ _returnvalue_2 _returnvalue_3)) _returnvalue_4) false "None"))
    (set `self.CurrentSpeed` _returnvalue_3)
    (set `self.AnimMoveVector` (`KismetMathLibrary.MakeVector` ActionValue_Y ActionValue_X)))
  (:`Completed`
    (goto _label_3)))

(event `EnhancedInput|/Game/Inputs/InputActions/Player/IA_Look`
  (params (ActionValue :type "Vector2D Structure") (ElapsedSeconds :type "Float (double-precision)") (TriggeredSeconds :type "Float (double-precision)") (InputAction :type "InputAction Object Reference" :default "/Game/Inputs/InputActions/Player/IA_Look.IA_Look"))
  (bind _capsulecollider (`self.CapsuleCollider`))
  (bind _camrot (`self.CamRot`))
  (:`Triggered`
    (`PrimitiveComponent.SetConstraintMode` _capsulecollider "None")
    (`SceneComponent.K2_AddLocalRotation` _capsulecollider (`KismetMathLibrary.MakeRotator` 0.0 0.0 ActionValue_X) false false)
    (`PrimitiveComponent.SetConstraintMode` _capsulecollider "SixDOF")
    (`SceneComponent.K2_SetRelativeRotation` _camrot (`KismetMathLibrary.MakeRotator` 0.0 (`KismetMathLibrary.FClamp` (+ (.pitch (`SceneComponent.RelativeRotation` _camrot)) ActionValue_Y) -70.0 80.0)) false false)))

(event `self.JumpDetector.OnComponentBeginOverlap`
  (params (OverlappedComponent :type "PrimitiveComponent Object Reference") (OtherActor :type "Actor Object Reference") (OtherComp :type "PrimitiveComponent Object Reference") (OtherBodyIndex :type Integer) (bFromSweep :type Boolean) (SweepResult :type "HitResult Structure (by ref)")))

(event `self.JumpDetector.OnComponentEndOverlap`
  (params (OverlappedComponent :type "PrimitiveComponent Object Reference") (OtherActor :type "Actor Object Reference") (OtherComp :type "PrimitiveComponent Object Reference") (OtherBodyIndex :type Integer)))

(event `Release`
  (bind _heldobject (`self.HeldObject`))
  (bind _capsulecollider (`self.CapsuleCollider`))
  (bind _sm_cube (`/Game/Blueprints/Cube/BP_Cube.SM_Cube` _heldobject))
  (`/Game/Blueprints/Cube/BP_Cube.Enable Physics` _heldobject :!label _label_4)
  (`PrimitiveComponent.SetPhysicsLinearVelocity` _sm_cube (`SceneComponent.GetComponentVelocity` _capsulecollider) false "None")
  (`PrimitiveComponent.SetPhysicsAngularVelocityInDegrees` _sm_cube (`PrimitiveComponent.GetPhysicsAngularVelocityInDegrees` _capsulecollider "None") false "None")
  (set `self.HeldObject` null)
  (set `self.IsHoldingState` 0))

(event `EnhancedInput|/Game/Inputs/InputActions/Player/IA_Grab`
  (params (ActionValue :type Boolean) (ElapsedSeconds :type "Float (double-precision)") (TriggeredSeconds :type "Float (double-precision)") (InputAction :type "InputAction Object Reference" :default "/Game/Inputs/InputActions/Player/IA_Grab.IA_Grab"))
  (bind _pickuppoint (`self.PickupPoint`))
  (bind _pointedobject (`self.PointedObject`))
  (bind _sm_cube (`/Game/Blueprints/Cube/BP_Cube.SM_Cube` (`self.HeldObject`)))
  (:`Triggered`
    (if (> (`self.IsHoldingState`) 1)
      (goto _label_4)
      (else
        (`/Engine/EditorBlueprintResources/StandardMacros.IsValid` _pointedobject
          (:`Is Valid`
            (`/Game/Blueprints/Cube/BP_Cube.Disable Physics` _pointedobject)
            (bind _output_get (set `self.HeldObject` _pointedobject))
            (set `self.PointedObject` null)
            (set `self.OldGrabPos` (`SceneComponent.K2_GetComponentToWorld` (`/Game/Blueprints/Cube/BP_Cube.SM_Cube` _output_get)))
            (set `self.IsHoldingState` 1)
            (bind (_direction _lerp) (`Timeline|Animate Grab` :!via `PlayFromStart`)
              (:`Update`
                (`SceneComponent.K2_SetWorldTransform` _sm_cube (`KismetMathLibrary.TLerp` (`self.OldGrabPos`) (`KismetMathLibrary.MakeTransform` (`SceneComponent.K2_GetComponentLocation` _pickuppoint) (`KismetMathLibrary.MakeRotFromX` (`SceneComponent.GetForwardVector` _pickuppoint))) _lerp) true true)
                (`PrimitiveComponent.SetPhysicsLinearVelocity` _sm_cube (0.0 0.0 0.0) false "None")
                (`PrimitiveComponent.SetPhysicsAngularVelocityInDegrees` _sm_cube (0.0 0.0 0.0) false "None"))
              (:`Finished`
                (set `self.IsHoldingState` 2))))
          (:`Is Not Valid`
            (`/Engine/EditorBlueprintResources/StandardMacros.IsValid` (`self.PointedAnomaly`)
              (:`Is Valid`
                (bind _asgm_state (cast `/Game/Blueprints/GameModes/GM_State` (`GameplayStatics.GetGameState`)))
                (`/Engine/EditorBlueprintResources/StandardMacros.IsValid` _asgm_state
                  (:`Is Valid`
                    (if (and (> (`/Game/Blueprints/GameModes/GM_State.AmountOfRiftMakers` _asgm_state) 0) (not (`/Game/Blueprints/Anomalies/BP_Anomaly.Enabled` (`self.PointedAnomaly`))))
                      (`/Game/Blueprints/GameModes/GM_State.Remove Rift Maker` _asgm_state)
                      (`/Game/Blueprints/Anomalies/BP_Anomaly.Open Anomaly` (`self.PointedAnomaly`)))))))))))))

(event `EnhancedInput|/Game/Inputs/InputActions/Player/IA_Throw`
  (params (ActionValue :type Boolean) (ElapsedSeconds :type "Float (double-precision)") (TriggeredSeconds :type "Float (double-precision)") (InputAction :type "InputAction Object Reference" :default "/Game/Inputs/InputActions/Player/IA_Throw.IA_Throw"))
  (bind _heldobject (`self.HeldObject`))
  (bind _capsulecollider (`self.CapsuleCollider`))
  (bind _sm_cube (`/Game/Blueprints/Cube/BP_Cube.SM_Cube` _heldobject))
  (:`Ongoing`
    (`/Game/Widgets/W_InGameUI.Set Crosshair Scale` (`self.UIWidget`) (+ (+ ElapsedSeconds 1.0) (* ElapsedSeconds 1.5))))
  (:`Canceled`
    (if (> (`self.IsHoldingState`) 1) :!label _label_5
      (`/Game/Blueprints/Cube/BP_Cube.Enable Physics` _heldobject)
      (`PrimitiveComponent.SetPhysicsLinearVelocity` _sm_cube (`SceneComponent.GetComponentVelocity` _capsulecollider) false "None")
      (`PrimitiveComponent.SetPhysicsAngularVelocityInDegrees` _sm_cube (`PrimitiveComponent.GetPhysicsAngularVelocityInDegrees` _capsulecollider "None") false "None")
      (`PrimitiveComponent.AddImpulse` _sm_cube (* (`SceneComponent.GetForwardVector` (`self.PickupPoint`)) (* ElapsedSeconds 500.0)) "None" true)
      (`/Game/Widgets/W_InGameUI.Set Crosshair Scale` (`self.UIWidget`) 0.0)
      (set `self.HeldObject` null)
      (set `self.IsHoldingState` 0)))
  (:`Completed`
    (goto _label_5)))

(event `EnhancedInput|/Game/Inputs/InputActions/Player/IA_Pause`
  (params (ActionValue :type Boolean) (ElapsedSeconds :type "Float (double-precision)") (TriggeredSeconds :type "Float (double-precision)") (InputAction :type "InputAction Object Reference" :default "/Game/Inputs/InputActions/Player/IA_Pause.IA_Pause"))
  (:`Triggered`
    (`/Game/Blueprints/GameModes/GM_State.Toggle Pause` (`self.GameState`))))

(event `Fade to Restart`
  (params (`Pause Menu` :type "/Game/Widgets/W_PauseMenu Object Reference"))
  (bind (_direction _newtrack_0) (`Timeline|Fade` :!via `PlayFromStart`)
    (:`Update`
      (`/Game/Widgets/W_PauseMenu.Fade` `Pause Menu` _newtrack_0))))

(event `Point UI`
  (bind _uiwidget (`self.UIWidget`))
  (if (== (`self.IsHoldingState`) 0)
    (bind (_direction _scale _is_point_mode) (`Timeline|UI Crosshair` :!label _label_6)
      (:`Update`
        (`/Engine/EditorBlueprintResources/StandardMacros.IsValid` _uiwidget
          (:`Is Valid`
            (`/Game/Widgets/W_InGameUI.Set Is Pointing` _uiwidget (`KismetMathLibrary.Conv_IntToBool` (`KismetMathLibrary.Round` _is_point_mode)))
            (`/Game/Widgets/W_InGameUI.Set Crosshair Scale` _uiwidget _scale)))))))

(event `Unpoint UI`
  (if (== (`self.IsHoldingState`) 0)
    (goto _label_6 :!via `Reverse`)))

(fn `ReorientPlayerAfterGravitySwitch`
  (returns (`New Rotation` :type "Rotator Structure"))
  (locals (MostAccurateRotation :type "Rotator Structure") (MostAccurateDot :type "Float (double-precision)" :default -1.0) (DebugLine :type "Float (double-precision)"))
  (bind _worldrot (`self.WorldRot`))
  (bind _returnvalue (`SceneComponent.K2_GetComponentRotation` _worldrot))
  (bind _returnvalue_2 (`KismetMathLibrary.Dot_VectorVector` (`KismetMathLibrary.Conv_RotatorToVector` _returnvalue) (`KismetMathLibrary.Conv_RotatorToVector` (`self.OldPlayerRotation`))))
  (for _ (range 360)
    (`SceneComponent.K2_AddLocalRotation` _worldrot (`KismetMathLibrary.MakeRotator` 0.0 0.0 1.0) false false)
    (if (> _returnvalue_2 (`local.MostAccurateDot`))
      (bind _output_get (set `local.MostAccurateDot` _returnvalue_2))
      (set `local.MostAccurateRotation` _returnvalue)))
  (return (`local.MostAccurateRotation`)))

(fn `UserConstructionScript`)