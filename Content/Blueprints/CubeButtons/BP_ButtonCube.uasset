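; Pressure button puzzle piece that tracks the mass of overlapping BP_Cubes and fires press or unpress calls around a trigger weight.
; Trigger overlaps add or remove clamped weight, wait for any running animation, then animate button depth and emission through a timeline.
; In letter mode, pressing also requires a matching cube character.
; The construction script sets colors and letter display; sounds follow time dilation and stay muted at startup.
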(event `Remove Weight`
  (params (Value :type "Float (double-precision)"))
  (bind _ispressed (`self.IsPressed`))
  (bind _currentweight (`self.CurrentWeight`))
  (if (> _currentweight 0.0)
    (set `self.CurrentWeight` (`KismetMathLibrary.FMax` (- _currentweight Value)))
    (if (not (< (`GameplayStatics.GetTimeSeconds`) 0.5))
      (`GameplayStatics.SpawnSoundAttached` "/Game/Audio/Buttons/A_Button_Out.A_Button_Out" (`self.Audio`) "None" (0.0 0.0 0.0) (struct) "KeepRelativeOffset" false 1.0 (`GameplayStatics.GetGlobalTimeDilation`) 0.0 "/Game/Audio/SoundAttenuationSettings.SoundAttenuationSettings" null))
    (if (`self.AnimRunning`) :!label _label
      (`KismetSystemLibrary.DelayUntilNextTick`)
      (goto _label)
      (else
        (`self.Update Weight`)
        (if (== (`self.TriggerWeight`) (`self.CurrentWeight`))
          (if _ispressed
            _
            (elif (`self.IsLetter`)
              (if (== (`self.Char`) (stale `Add Weight` `Character (if any)`))
                (set `self.IsPressed` true :!label _label_2)
                (`self.OnPress`))
              (else
                (goto _label_2))))
          (elif _ispressed
            (set `self.IsPressed` false)
            (`self.OnUnpress`)))))))

(event `Add Weight`
  (params (value :type "Float (double-precision)") (`Character (if any)` :type Text))
  (bind _currentweight (`self.CurrentWeight`))
  (bind _triggerweight (`self.TriggerWeight`))
  (if (< _currentweight _triggerweight)
    (set `self.CurrentWeight` (`KismetMathLibrary.FMin` (+ _currentweight value) _triggerweight))
    (if (< (`GameplayStatics.GetTimeSeconds`) 0.5)
      (goto _label)
      (else
        (`GameplayStatics.SpawnSoundAttached` "/Game/Audio/Buttons/A_Button_In.A_Button_In" (`self.Audio`) "None" (0.0 0.0 0.0) (struct) "KeepRelativeOffset" false 1.0 (`GameplayStatics.GetGlobalTimeDilation`) 0.0 "/Game/Audio/SoundAttenuationSettings.SoundAttenuationSettings" null)
        (goto _label)))))

(event `Update Weight`
  (bind _triggerweight (`self.TriggerWeight`))
  (bind _returnvalue (/ (`self.CurrentWeightSaved`) _triggerweight))
  (bind _returnvalue_2 (/ (`KismetMathLibrary.FClamp` (`self.CurrentWeight`) 0.0 _triggerweight) _triggerweight))
  (set `self.AnimRunning` true)
  (bind (_direction _out _emissive) (`Timeline|Pressing` :!via `PlayFromStart`)
    (:`Update`
      (`SceneComponent.K2_SetRelativeLocation` (`self.SM_Button_One_Button`) (`KismetMathLibrary.MakeVector` 0.0 0.0 (* (`KismetMathLibrary.Lerp` _returnvalue _returnvalue_2 _out) -7.5)) false false)
      (`MaterialInstanceDynamic.SetScalarParameterValue` (`self.Mat`) "Emission Intensity" (`KismetMathLibrary.Lerp` _returnvalue _returnvalue_2 _emissive)))
    (:`Finished`
      (set `self.CurrentWeightSaved` (`self.CurrentWeight`))
      (set `self.AnimRunning` false))))

(event `self.Trigger.OnComponentBeginOverlap`
  (params (OverlappedComponent :type "PrimitiveComponent Object Reference") (OtherActor :type "Actor Object Reference") (OtherComp :type "PrimitiveComponent Object Reference") (OtherBodyIndex :type Integer) (bFromSweep :type Boolean) (SweepResult :type "HitResult Structure (by ref)"))
  (bind _returnvalue (`PrimitiveComponent.GetCollisionObjectType` OtherComp))
  (if (or (`|EnumEquality` _returnvalue "ECC_WorldDynamic") (`|EnumEquality` _returnvalue "ECC_PhysicsBody") (`|EnumEquality` _returnvalue "ECC_Vehicle"))
    (bind _asbp_cube (cast `/Game/Blueprints/Cube/BP_Cube` OtherActor))
    (`self.Add Weight` (`PrimitiveComponent.GetMass` OtherComp) (`/Game/Blueprints/Cube/BP_Cube.Char` _asbp_cube))))

(event `self.Trigger.OnComponentEndOverlap`
  (params (OverlappedComponent :type "PrimitiveComponent Object Reference") (OtherActor :type "Actor Object Reference") (OtherComp :type "PrimitiveComponent Object Reference") (OtherBodyIndex :type Integer))
  (bind _returnvalue (`PrimitiveComponent.GetCollisionObjectType` OtherComp))
  (if (or (`|EnumEquality` _returnvalue "ECC_WorldDynamic") (`|EnumEquality` _returnvalue "ECC_PhysicsBody") (`|EnumEquality` _returnvalue "ECC_Vehicle"))
    (`self.Remove Weight` (`PrimitiveComponent.GetMass` OtherComp))))

(fn `UserConstructionScript`
  (bind _sm_button_one_button (`self.SM_Button_One_Button`))
  (bind _letter (`self.Letter`))
  (bind _returnvalue (`PrimitiveComponent.CreateDynamicMaterialInstance` _sm_button_one_button 0 (`PrimitiveComponent.GetMaterial` _sm_button_one_button 0) "None"))
  (bind _output_get (set `self.Mat` _returnvalue))
  (`MaterialInstanceDynamic.SetVectorParameterValue` _output_get "Tint" (`self.ButtonColor`))
  (`MaterialInstanceDynamic.SetVectorParameterValue` _output_get "Emission Tint" (`self.ButtonColorEmi`))
  (if (`self.IsLetter`)
    (`SceneComponent.SetVisibility` _letter true true)
    (set `Text3DComponent.Text` (`self.Char`) (`self.Char1`))
    (if (`self.HideLetter`)
      (`SceneComponent.SetVisibility` (`self.Char1`) false false))
    (else
      (`SceneComponent.SetVisibility` _letter false true))))