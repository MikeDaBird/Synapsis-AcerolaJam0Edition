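; BP_Anomaly is a rift that can open and close and sends the player into an anomaly of its Type.
; Open and close events drive a scaling timeline, smoke, sound and the RiftMakerTrigger collision, which is active only while closed.
; When enabled, capsule overlap by BP_PlayerRig has GM_State load the anomaly and apply a time-dilation effect, guarded by a transition flag.
; The construction script tints material, smoke and light from SmokeColor.
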(event `self.ReceiveBeginPlay`
  (bind _asgm_state (cast `/Game/Blueprints/GameModes/GM_State` (`GameplayStatics.GetGameState`)))
  (`/Engine/EditorBlueprintResources/StandardMacros.IsValid` _asgm_state
    (:`Is Valid`
      (set `self.GameState` _asgm_state)
      (if (not (`self.Enabled`))
        (bind (_direction _scale_out) (`Timeline|Anomaly Scaling` :`NewTime` 0.6 :!via `SetNewTime` :!label _label)
          (:`Update`
            (`SceneComponent.SetRelativeScale3D` (`self.SM_Anomaly`) _scale_out)))))))

(event `Open Anomaly`
  (if (not (`self.Enabled`))
    (set `self.Enabled` true)
    (`GameplayStatics.SpawnSoundAttached` "/Game/Audio/Anomalies/A_Anomaly_Open.A_Anomaly_Open" (`self.MS_Anomaly_Ambient`) "None" (0.0 0.0 0.0) (struct) "KeepRelativeOffset" false 1.0 1.0 0.0 null null)
    (`PrimitiveComponent.SetCollisionEnabled` (`self.RiftMakerTrigger`) "NoCollision")
    (`NiagaraComponent.SetVariableFloat` (`self.NS_AnomalySmoke_Volume`) "Spawn Rate" 20.0)
    (goto _label :!via `Reverse`)))

(event `Close Anomaly`
  (if (`self.Enabled`)
    (set `self.Enabled` false)
    (`GameplayStatics.SpawnSoundAttached` "/Game/Audio/Anomalies/A_Anomaly_Open.A_Anomaly_Open" (`self.MS_Anomaly_Ambient`) "None" (0.0 0.0 0.0) (struct) "KeepRelativeOffset" false 1.0 0.6 0.0 null null)
    (`PrimitiveComponent.SetCollisionEnabled` (`self.RiftMakerTrigger`) "QueryOnly")
    (`NiagaraComponent.SetVariableFloat` (`self.NS_AnomalySmoke_Volume`) "Spawn Rate" 0.0)
    (goto _label)))

(event `self.Capsule.OnComponentBeginOverlap`
  (params (OverlappedComponent :type "PrimitiveComponent Object Reference") (OtherActor :type "Actor Object Reference") (OtherComp :type "PrimitiveComponent Object Reference") (OtherBodyIndex :type Integer) (bFromSweep :type Boolean) (SweepResult :type "HitResult Structure (by ref)"))
  (bind _gamestate (`self.GameState`))
  (bind _gamestate_2 (`self.GameState`))
  (if (`self.Enabled`)
    (bind _asbp_player_rig (cast `/Game/Blueprints/Player/Rig/BP_PlayerRig` OtherActor))
    (`/Engine/EditorBlueprintResources/StandardMacros.IsValid` _asbp_player_rig
      (:`Is Valid`
        (if (not (or (`/Game/Blueprints/GameModes/GM_State.TransitionningAnomaly` _gamestate_2) (not (`KismetSystemLibrary.IsValid` _gamestate_2))))
          (set `/Game/Blueprints/GameModes/GM_State.TransitionningAnomaly` true _gamestate_2)
          (`/Game/Blueprints/GameModes/GM_State.Load Anomaly of Type` _gamestate (`self.Type`))
          (`/Game/Blueprints/GameModes/GM_State.Effect Enter Anomaly` _gamestate (`self.TimeDilation`))
          (`GameplayStatics.SpawnSoundAttached` "/Game/Audio/Anomalies/A_Anomaly_Enter.A_Anomaly_Enter" (`self.MS_Anomaly_Ambient`) "None" (`self.K2_GetActorLocation`) (struct) "KeepRelativeOffset" false 0.65 1.0 0.0 null null)
          (bind _returnvalue (`GameUserSettings.GetGameUserSettings`))
          (`GameUserSettings.ApplyNonResolutionSettings` _returnvalue))))))

(event `self.Capsule.OnComponentEndOverlap`
  (params (OverlappedComponent :type "PrimitiveComponent Object Reference") (OtherActor :type "Actor Object Reference") (OtherComp :type "PrimitiveComponent Object Reference") (OtherBodyIndex :type Integer))
  (`KismetSystemLibrary.Delay` (* (`GameplayStatics.GetGlobalTimeDilation`) 0.2))
  (bind _asbp_player_rig (cast `/Game/Blueprints/Player/Rig/BP_PlayerRig` OtherActor))
  (`/Engine/EditorBlueprintResources/StandardMacros.IsValid` _asbp_player_rig
    (:`Is Valid`
      (set `/Game/Blueprints/GameModes/GM_State.TransitionningAnomaly` false (`self.GameState`)))))

(fn `UserConstructionScript`
  (bind _smokecolor (`self.SmokeColor`))
  (bind _returnvalue (`PrimitiveComponent.CreateDynamicMaterialInstance` (`self.SM_Anomaly`) 0 (`self.AnomalyMat`) "None"))
  (bind _output_get (set `self.Mat` _returnvalue))
  (`MaterialInstanceDynamic.SetVectorParameterValue` _output_get "Offset" (`KismetMathLibrary.Conv_VectorToLinearColor` (`self.K2_GetActorLocation`)))
  (`MaterialInstanceDynamic.SetVectorParameterValue` _output_get "Tint" (`self.SmokeColor`))
  (`NiagaraComponent.SetVariableLinearColor` (`self.NS_AnomalySmoke_Volume`) "Smoke Color" _smokecolor)
  (`LightComponent.SetLightColor` (`self.PointLight`) _smokecolor true)
  (if (not (`self.Enabled`))
    (`SceneComponent.SetRelativeScale3D` (`self.SM_Anomaly`) (0.03 0.03 0.7))
    (`PrimitiveComponent.SetCollisionEnabled` (`self.RiftMakerTrigger`) "QueryOnly")
    (`NiagaraComponent.SetVariableFloat` (`self.NS_AnomalySmoke_Volume`) "Spawn Rate" 0.0)))