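; BP_RespawnZone is a trigger volume that restarts the level when the player rig enters it.
; On BeginPlay it caches the game state as GM_State.
; When a BP_PlayerRig begins overlapping its Box component, it calls RestartLevel on that game state unless the IsDed flag is already set.
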(event `self.ReceiveBeginPlay`
  (bind _asgm_state (cast `/Game/Blueprints/GameModes/GM_State` (`GameplayStatics.GetGameState`)))
  (`/Engine/EditorBlueprintResources/StandardMacros.IsValid` _asgm_state
    (:`Is Valid`
      (set `self.Game State` _asgm_state))))

(event `self.Box.OnComponentBeginOverlap`
  (params (OverlappedComponent :type "PrimitiveComponent Object Reference") (OtherActor :type "Actor Object Reference") (OtherComp :type "PrimitiveComponent Object Reference") (OtherBodyIndex :type Integer) (bFromSweep :type Boolean) (SweepResult :type "HitResult Structure (by ref)"))
  (bind _asbp_player_rig (cast `/Game/Blueprints/Player/Rig/BP_PlayerRig` OtherActor))
  (`/Engine/EditorBlueprintResources/StandardMacros.IsValid` _asbp_player_rig
    (:`Is Valid`
      (if (not (`/Game/Blueprints/GameModes/GM_State.IsDed` (`self.Game State`)))
        (`/Game/Blueprints/GameModes/GM_State.Restart Level` (`self.Game State`))))))

(fn `UserConstructionScript`)