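; Anomaly actor that randomly swaps between a standard and an anomalized child actor when the player looks away.
; The construction script sets both child actors' classes, applying configured meshes for static or skeletal mesh actors.
; Tick projects IsVisibleTester's eight box corners to screen; when all stop projecting, it rerolls against ChancesToSwap, toggling visibility and scale.
; Line-trace occlusion checks and initial-scale capture are disconnected.
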(event `RandomizeAnomaly`
  (bind _standard (`self.Standard`))
  (bind _anomalized (`self.Anomalized`))
  (bind _standard_2 (`self.Standard`))
  (bind _anomalized_2 (`self.Anomalized`))
  (if (<= (`KismetMathLibrary.RandomFloat`) (`self.ChancesToSwap`))
    (`SceneComponent.SetVisibility` _anomalized true false)
    (`SceneComponent.SetVisibility` _standard false false)
    (`SceneComponent.SetRelativeScale3D` _standard_2 (0.0 0.0 0.0))
    (`SceneComponent.SetRelativeScale3D` _anomalized_2 (`self.Init Scale Anomaly`))
    (else
      (`SceneComponent.SetVisibility` _standard true false)
      (`SceneComponent.SetVisibility` _anomalized false false)
      (`SceneComponent.SetRelativeScale3D` _anomalized_2 (0.0 0.0 0.0))
      (`SceneComponent.SetRelativeScale3D` _standard_2 (`self.Init Scale Regular`)))))

(event `self.ReceiveBeginPlay`
  (`SceneComponent.SetVisibility` (`self.Anomalized`) false false))

(event `self.ReceiveTick`
  (params (DeltaSeconds :type "Float (single-precision)"))
  (bind _isvisibletester (`self.IsVisibleTester`))
  (bind _returnvalue (`SceneComponent.K2_GetComponentLocation` _isvisibletester))
  (bind _x (.x (`SceneComponent.K2_GetComponentScale` _isvisibletester)))
  (bind _y (.y (`SceneComponent.K2_GetComponentScale` _isvisibletester)))
  (bind _z (.z (`SceneComponent.K2_GetComponentScale` _isvisibletester)))
  (bind _returnvalue_2 (* _z -1.0))
  (bind _returnvalue_3 (* _x -1.0))
  (bind _returnvalue_4 (* _y -1.0))
  (bind _returnvalue_5 (or (`.ReturnValue` (`GameplayStatics.ProjectWorldToScreen` (`GameplayStatics.GetPlayerController` 0) (+ _returnvalue (`KismetMathLibrary.MakeVector` _x _y _z)) true)) (`.ReturnValue` (`GameplayStatics.ProjectWorldToScreen` null (+ _returnvalue (`KismetMathLibrary.MakeVector` _returnvalue_3 _y _z)) true)) (`.ReturnValue` (`GameplayStatics.ProjectWorldToScreen` null (+ _returnvalue (`KismetMathLibrary.MakeVector` _x _returnvalue_4 _z)) true)) (`.ReturnValue` (`GameplayStatics.ProjectWorldToScreen` null (+ _returnvalue (`KismetMathLibrary.MakeVector` _returnvalue_3 _returnvalue_4 _z)) true)) (`.ReturnValue` (`GameplayStatics.ProjectWorldToScreen` null (+ _returnvalue (`KismetMathLibrary.MakeVector` _x _y _returnvalue_2)) true)) (`.ReturnValue` (`GameplayStatics.ProjectWorldToScreen` null (+ _returnvalue (`KismetMathLibrary.MakeVector` _returnvalue_3 _y _returnvalue_2)) true)) (`.ReturnValue` (`GameplayStatics.ProjectWorldToScreen` null (+ _returnvalue (`KismetMathLibrary.MakeVector` _x _returnvalue_4 _returnvalue_2)) true)) (`.ReturnValue` (`GameplayStatics.ProjectWorldToScreen` null (+ _returnvalue (`KismetMathLibrary.MakeVector` _returnvalue_3 _returnvalue_4 _returnvalue_2)) true))))
  (if (not (== (`self.VisibilityTrigger`) _returnvalue_5))
    (bind _output_get (set `self.VisibilityTrigger` _returnvalue_5))
    (if (not _output_get)
      (`self.RandomizeAnomaly`))))

(fn `UserConstructionScript`
  (bind _regular_class (`self.Regular Class`))
  (bind _anomaly_class (`self.Anomaly Class`))
  (`ChildActorComponent.SetChildActorClass` (`self.Standard`) _regular_class)
  (`ChildActorComponent.SetChildActorClass` (`self.Anomalized`) (`self.Anomaly Class`))
  (if (== _regular_class "/Script/Engine.StaticMeshActor")
    (bind _asstatic_mesh_actor (cast `StaticMeshActor` (`ChildActorComponent.ChildActor` (`self.Standard`)))
      (:`then`
        (bind _staticmeshcomponent (`StaticMeshActor.StaticMeshComponent` _asstatic_mesh_actor))
        (`StaticMeshComponent.SetStaticMesh` _staticmeshcomponent (`self.Regular Mesh`))
        (`PrimitiveComponent.SetPhysMaterialOverride` _staticmeshcomponent (`self.Regular PhysMat`))
        (set `PrimitiveComponent.bGenerateOverlapEvents` true _staticmeshcomponent))
      (:`CastFailed`
        _)))
  (if (== _regular_class "/Script/Engine.SkeletalMeshActor")
    (bind _asskeletal_mesh_actor (cast `SkeletalMeshActor` (`ChildActorComponent.ChildActor` (`self.Standard`)))
      (:`then`
        (`SkeletalMeshComponent.SetSkeletalMeshAsset` (`SkeletalMeshActor.SkeletalMeshComponent` _asskeletal_mesh_actor) (`self.Regular SkeletalMesh`)))
      (:`CastFailed`
        _)))
  (if (== _anomaly_class "/Script/Engine.StaticMeshActor")
    (bind _asstatic_mesh_actor_2 (cast `StaticMeshActor` (`ChildActorComponent.ChildActor` (`self.Anomalized`)))
      (:`then`
        (bind _staticmeshcomponent_2 (`StaticMeshActor.StaticMeshComponent` _asstatic_mesh_actor_2))
        (`StaticMeshComponent.SetStaticMesh` _staticmeshcomponent_2 (`self.Anomaly Mesh`))
        (`PrimitiveComponent.SetPhysMaterialOverride` _staticmeshcomponent_2 (`self.Anomaly PhysMat`))
        (set `PrimitiveComponent.bGenerateOverlapEvents` true _staticmeshcomponent_2))
      (:`CastFailed`
        _)))
  (if (== _anomaly_class "/Script/Engine.SkeletalMeshActor")
    (bind _asskeletal_mesh_actor_2 (cast `SkeletalMeshActor` (`ChildActorComponent.ChildActor` (`self.Anomalized`))))
    (`SkeletalMeshComponent.SetSkeletalMeshAsset` (`SkeletalMeshActor.SkeletalMeshComponent` _asskeletal_mesh_actor_2) (`self.Anomaly SkeletalMesh`))))