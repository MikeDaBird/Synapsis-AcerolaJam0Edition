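; BP_GravityFloor is a trigger volume that changes the player rig's gravity direction on overlap.
; The construction script stores the Box's forward vector as GravityVector, so the box's orientation defines the gravity direction.
; When a BP_PlayerRig begins overlapping the box with a different gravity vector, it receives this one and calls UpdateGravityVector to apply it.
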(event `self.Box.OnComponentBeginOverlap`
  (params (OverlappedComponent :type "PrimitiveComponent Object Reference") (OtherActor :type "Actor Object Reference") (OtherComp :type "PrimitiveComponent Object Reference") (OtherBodyIndex :type Integer) (bFromSweep :type Boolean) (SweepResult :type "HitResult Structure (by ref)"))
  (bind _gravityvector (`self.GravityVector`))
  (bind _asbp_player_rig (cast `/Game/Blueprints/Player/Rig/BP_PlayerRig` OtherActor))
  (`/Engine/EditorBlueprintResources/StandardMacros.IsValid` _asbp_player_rig
    (:`Is Valid`
      (if (not (== _gravityvector (`/Game/Blueprints/Player/Rig/BP_PlayerRig.GravityVector` _asbp_player_rig) :`ErrorTolerance` 0.0001))
        (set `/Game/Blueprints/Player/Rig/BP_PlayerRig.GravityVector` _gravityvector _asbp_player_rig)
        (`/Game/Blueprints/Player/Rig/BP_PlayerRig.UpdateGravityVector` _asbp_player_rig)))))

(fn `UserConstructionScript`
  (set `self.GravityVector` (`SceneComponent.GetForwardVector` (`self.Box`))))