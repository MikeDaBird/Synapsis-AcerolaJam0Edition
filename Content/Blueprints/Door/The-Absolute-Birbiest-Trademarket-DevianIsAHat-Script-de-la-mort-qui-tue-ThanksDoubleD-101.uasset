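; Sliding double-door actor that opens when enough linked buttons are pressed and closes when the count drops below the threshold.
; BeginPlay binds each button's press/unpress events to a counter driving OpenDoor/CloseDoor; InvertedSetup swaps their animations and starts the door open.
; Timelines slide both panels apart or together, reversing if interrupted mid-animation.
; Sounds follow time dilation and are muted during startup; the construction script toggles frame visibility.
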(event `self.ReceiveBeginPlay`
  (for _array_element (`self.LinkedButtons`)
    (add `/Game/Blueprints/CubeButtons/BP_ButtonCube.OnPress` _array_element (delegate `Press`))
    (add `/Game/Blueprints/CubeButtons/BP_ButtonCube.OnUnpress` _array_element (delegate `Unpress`)))
  (if (`self.InvertedSetup`)
    (`self.Close Door`)))

(event `Press`
  (bind _opened (`self.Opened`))
  (set `self.CountedValidElements` (+ (`self.CountedValidElements`) 1))
  (if (>= (`self.CountedValidElements`) (`self.ValidElementsToCount`)) :!label _label
    (if (not _opened)
      (`self.Open Door`))
    (elif _opened
      (`self.Close Door`))))

(event `Unpress`
  (set `self.CountedValidElements` (- (`self.CountedValidElements`) 1))
  (goto _label))

(event `Open Door`
  (bind _returnvalue (`GameplayStatics.GetGlobalTimeDilation`))
  (bind _audio (`self.Audio`))
  (bind _returnvalue_2 (< (`GameplayStatics.GetTimeSeconds`) 0.5))
  (set `self.Opened` true)
  (if (`self.InvertedSetup`)
    (if (`self.AnimPlaying`) :!label _label_2
      (bind (_direction _open) (`Timeline|CloseDoor` :!via `Reverse` :!label _label_3)
        (:`Update`
          (bind _returnvalue_3 (* _open 100.0))
          (`SceneComponent.K2_SetRelativeLocation` (`self.DoorL`) (`KismetMathLibrary.MakeVector` (* _returnvalue_3 -1.0)) false false)
          (`SceneComponent.K2_SetRelativeLocation` (`self.DoorR`) (`KismetMathLibrary.MakeVector` _returnvalue_3) false false))
        (:`Finished`
          (set `self.AnimPlaying` false :!label _label_4)))
      (else
        (set `self.AnimPlaying` true)
        (if _returnvalue_2
          (goto _label_3 :!via `PlayFromStart`)
          (else
            (`GameplayStatics.SpawnSoundAttached` "/Game/Audio/Doors/A_Door_Closed.A_Door_Closed" _audio "None" (0.0 0.0 0.0) (struct) "KeepRelativeOffset" false 1.0 _returnvalue 0.0 "/Game/Audio/SoundAttenuationSettings.SoundAttenuationSettings" null)
            (goto _label_3 :!via `PlayFromStart`)))))
    (else
      (if (`self.AnimPlaying`) :!label _label_5
        (bind (_direction_2 _open_2) (`Timeline|OpenDoor` :!via `Reverse` :!label _label_6)
          (:`Update`
            (bind _returnvalue_4 (* _open_2 100.0))
            (`SceneComponent.K2_SetRelativeLocation` (`self.DoorL`) (`KismetMathLibrary.MakeVector` (* _returnvalue_4 -1.0)) false false)
            (`SceneComponent.K2_SetRelativeLocation` (`self.DoorR`) (`KismetMathLibrary.MakeVector` _returnvalue_4) false false))
          (:`Finished`
            (goto _label_4)))
        (else
          (set `self.AnimPlaying` true)
          (if _returnvalue_2
            (goto _label_6 :!via `PlayFromStart`)
            (else
              (`GameplayStatics.SpawnSoundAttached` "/Game/Audio/Doors/A_Door_Open.A_Door_Open" _audio "None" (0.0 0.0 0.0) (struct) "KeepRelativeOffset" false 1.0 _returnvalue 0.0 "/Game/Audio/SoundAttenuationSettings.SoundAttenuationSettings" null)
              (goto _label_6 :!via `PlayFromStart`))))))))

(event `Close Door`
  (set `self.Opened` false)
  (if (`self.InvertedSetup`)
    (goto _label_5)
    (else
      (goto _label_2))))

(fn `UserConstructionScript`
  (`SceneComponent.SetVisibility` (`self.DoorFrame`) (`self.ShowFrame`) false))