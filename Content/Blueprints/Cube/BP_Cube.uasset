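; BP_Cube is a physics cube that can optionally serve as a letter block, with its construction script copying one character to six text components.
; DisablePhysics turns off gravity, applies a slippery material and ignores Pawn, Destructible and Vehicle collisions; EnablePhysics restores them and wakes the body next tick.
; Hard hits after startup spawn an impact sound, pitched by time dilation and fed a force parameter from the impulse.
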(event `Disable Physics`
  (bind _sm_cube (`self.SM_Cube`))
  (`PrimitiveComponent.SetEnableGravity` _sm_cube false)
  (`PrimitiveComponent.SetPhysMaterialOverride` _sm_cube "/Game/PhysicsMats/PhysMat_SlidyBoi.PhysMat_SlidyBoi")
  (`PrimitiveComponent.SetCollisionResponseToChannel` _sm_cube "ECC_Pawn" "ECR_Ignore")
  (`PrimitiveComponent.SetCollisionResponseToChannel` _sm_cube "ECC_Destructible" "ECR_Ignore")
  (`PrimitiveComponent.SetCollisionResponseToChannel` _sm_cube "ECC_Vehicle" "ECR_Ignore"))

(event `Enable Physics`
  (bind _sm_cube (`self.SM_Cube`))
  (`PrimitiveComponent.SetEnableGravity` _sm_cube true)
  (`PrimitiveComponent.SetPhysMaterialOverride` _sm_cube (`self.PhysMat`))
  (`PrimitiveComponent.SetCollisionResponseToChannel` _sm_cube "ECC_Pawn" "ECR_Block")
  (`PrimitiveComponent.SetCollisionResponseToChannel` (`self.SM_Cube`) "ECC_Destructible" "ECR_Block")
  (`PrimitiveComponent.SetCollisionResponseToChannel` _sm_cube "ECC_Vehicle" "ECR_Block")
  (`KismetSystemLibrary.DelayUntilNextTick`)
  (`PrimitiveComponent.WakeAllRigidBodies` _sm_cube))

(event `self.SM_Cube.OnComponentHit`
  (params (HitComponent :type "PrimitiveComponent Object Reference") (OtherActor :type "Actor Object Reference") (OtherComp :type "PrimitiveComponent Object Reference") (NormalImpulse :type "Vector Structure") (Hit :type "HitResult Structure (by ref)"))
  (bind _returnvalue (/ (`KismetMathLibrary.VSize` NormalImpulse) 60000.0))
  (if (and (> (`GameplayStatics.GetTimeSeconds`) 0.5) (> _returnvalue 0.3))
    (bind _returnvalue_2 (`GameplayStatics.SpawnSoundAtLocation` (`self.CubeSounds`) (`.ImpactPoint` (`GameplayStatics.BreakHitResult` Hit)) (struct) 1.0 (`GameplayStatics.GetGlobalTimeDilation`) 0.0 "/Game/Audio/SoundAttenuationSettings.SoundAttenuationSettings" null))
    (`AudioComponent.SetFloatParameter` _returnvalue_2 "Force" (- _returnvalue 0.3))))

(fn `UserConstructionScript`
  (bind _letter (`self.Letter`))
  (bind _char (`self.Char`))
  (`PrimitiveComponent.SetPhysMaterialOverride` (`self.SM_Cube`) (`self.PhysMat`))
  (if (`self.IsLetter`)
    (`SceneComponent.SetVisibility` _letter true true)
    (set `Text3DComponent.Text` _char (`self.Char1`))
    (set `Text3DComponent.Text` _char (`self.Char2`))
    (set `Text3DComponent.Text` _char (`self.Char3`))
    (set `Text3DComponent.Text` _char (`self.Char4`))
    (set `Text3DComponent.Text` _char (`self.Char5`))
    (set `Text3DComponent.Text` _char (`self.Char6`))
    (else
      (`SceneComponent.SetVisibility` _letter false true))))