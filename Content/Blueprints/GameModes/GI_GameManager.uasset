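; Game instance for a puzzle game that holds level progression, player settings and speedrun timing across levels.
; Init restores progress, best time and settings from a save slot, Shutdown writes them back, and Init or ManualInit creates the fade post-process material instance.
; NextLevel advances through GameLevels, raising the unlock cap and returning to the main menu when the run completes.
; The speedrun timer adds real-time deltas to a stored offset; its pause event is empty.
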(event `Manual Init`
  (if (not (`KismetSystemLibrary.IsValid` (`self.FadeMat`)))
    (bind _returnvalue (`KismetMaterialLibrary.CreateDynamicMaterialInstance` (`self.FadeMatMain`) "MID_FadePP" :!label _label))
    (bind _output_get (set `self.FadeMat` _returnvalue))))

(event `self.ReceiveInit`
  (bind _returnvalue (`GameplayStatics.LoadGameFromSlot` "MDB_UnrealPuzzle_Save"))
  (bind _asgm_game_save (cast `/Game/Blueprints/GameModes/GM_GameSave` _returnvalue)
    (:`then`
      (set `self.MaxLevelUnlock` (`/Game/Blueprints/GameModes/GM_GameSave.MaxLevelReached` _asgm_game_save))
      (set `self.Best Time Saved` (`/Game/Blueprints/GameModes/GM_GameSave.BestSpeedTime` _asgm_game_save))
      (set `self.Quality` (`/Game/Blueprints/GameModes/GM_GameSave.Quality` _asgm_game_save))
      (set `self.Fullscreen` (`/Game/Blueprints/GameModes/GM_GameSave.Fullscreen` _asgm_game_save))
      (set `self.RenderResScale` (`/Game/Blueprints/GameModes/GM_GameSave.RenderResScale` _asgm_game_save))
      (set `self.JPEGMODE` (`/Game/Blueprints/GameModes/GM_GameSave.JPEGMODE` _asgm_game_save))
      (set `self.DisplaySpeedrunTimer` (`/Game/Blueprints/GameModes/GM_GameSave.DisplaySpeedrunTimer` _asgm_game_save))
      (set `self.VolumeMaster` (`/Game/Blueprints/GameModes/GM_GameSave.VolumeMaster` _asgm_game_save))
      (set `self.VolumeMusic` (`/Game/Blueprints/GameModes/GM_GameSave.VolumeMusic` _asgm_game_save))
      (set `self.VolumeSFX` (`/Game/Blueprints/GameModes/GM_GameSave.VolumeSFX` _asgm_game_save))
      (`|LoadAsset` "/Game/Audio/Anomalies/A_Anomaly_Enter.A_Anomaly_Enter"
        (:`then`
          (goto _label))))
    (:`CastFailed`
      (goto _label))))

(event `Load Level`
  (params (name :type Name))
  (`GameplayStatics.OpenLevel` name))

(event `Next Level`
  (bind _returnvalue (`KismetArrayLibrary.Array_Length` (`self.GameLevels`)))
  (bind _output_get (set `self.CurrentLevelIndex` (+ (`self.CurrentLevelIndex`) 1)))
  (set `self.MaxLevelUnlock` (`KismetMathLibrary.Min` (`KismetMathLibrary.Max` _output_get (`self.MaxLevelUnlock`)) _returnvalue))
  (if (>= _output_get _returnvalue)
    (set `self.RunCompleted` true)
    (`self.Load Level` "l_MainMenu")
    (else
      (`self.Load Level` (`KismetStringLibrary.Conv_StringToName` (`|GetArrayItem` (`self.GameLevels`) _output_get))))))

(event `self.ReceiveShutdown`
  (bind _returnvalue (`GameplayStatics.CreateSaveGameObject` "/Game/Blueprints/GameModes/GM_GameSave.GM_GameSave_C"))
  (bind _output_get (set `self.SaveGameInstance` _returnvalue))
  (set `/Game/Blueprints/GameModes/GM_GameSave.MaxLevelReached` (`self.MaxLevelUnlock`) _output_get)
  (set `/Game/Blueprints/GameModes/GM_GameSave.BestSpeedTime` (`self.Best Time Saved`) _output_get)
  (set `/Game/Blueprints/GameModes/GM_GameSave.Quality` (`self.Quality`) _output_get)
  (set `/Game/Blueprints/GameModes/GM_GameSave.Fullscreen` (`self.Fullscreen`) _output_get)
  (set `/Game/Blueprints/GameModes/GM_GameSave.RenderResScale` (`self.RenderResScale`) _output_get)
  (set `/Game/Blueprints/GameModes/GM_GameSave.JPEGMODE` (`self.JPEGMODE`) _output_get)
  (set `/Game/Blueprints/GameModes/GM_GameSave.DisplaySpeedrunTimer` (`self.DisplaySpeedrunTimer`) _output_get)
  (set `/Game/Blueprints/GameModes/GM_GameSave.VolumeMaster` (`self.VolumeMaster`) _output_get)
  (set `/Game/Blueprints/GameModes/GM_GameSave.VolumeMusic` (`self.VolumeMusic`) _output_get)
  (set `/Game/Blueprints/GameModes/GM_GameSave.VolumeSFX` (`self.VolumeSFX`) _returnvalue)
  (`GameplayStatics.SaveGameToSlot` _output_get "MDB_UnrealPuzzle_Save"))

(event `Run Speedrun Timer`
  (bind (_seconds _partialseconds) (`GameplayStatics.GetAccurateRealTime`))
  (set `self.SpeedrunTimerStartedTime` (+ _seconds _partialseconds))
  (set `self.SpeedrunTimerAdder` (`self.SpeedrunTimer`)))

(event `Update Speedrun Timer`
  (bind (_seconds _partialseconds) (`GameplayStatics.GetAccurateRealTime`))
  (set `self.SpeedrunTimer` (+ (- (+ _seconds _partialseconds) (`self.SpeedrunTimerStartedTime`)) (`self.SpeedrunTimerAdder`))))

(event `Pause Speedrun Timer`)

(event `Reset Speedrun Timer`
  (set `self.SpeedrunTimer` 0.0)
  (set `self.SpeedrunTimerStartedTime` 0.0)
  (set `self.SpeedrunTimerAdder` 0.0))