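; GM_State runs a level's anomaly variants, time dilation, pause menu and restart or next-level transitions.
; UpdateLevels streams in every variant and repositions the player; LoadAnomalyofType swaps visibility by name suffix, avoiding reloads.
; Time changes counter-scale player dilation and ease music pitch, while anomaly entry pulses post-process effects.
; Transitions fade a filter-colored post-process material before GI_GameManager loads levels; pausing also halts its speedrun timer.
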(event `Update Levels`
  (params (`Level Normal` :type "World Soft Object Reference") (`Level Time Speed` :type "World Soft Object Reference") (`Level Time Travel` :type "World Soft Object Reference") (`Level Color 1` :type "World Soft Object Reference") (`Level Color 2` :type "World Soft Object Reference") (`Level Color 3` :type "World Soft Object Reference") (`Level Color 4` :type "World Soft Object Reference") (`Level Uncanny` :type "World Soft Object Reference") (`Level Abnormal` :type "World Soft Object Reference") (`Level Name Prefix` :type String) (`Player Spawn` :type "Transform Structure"))
  (bind _fadeppmaterial (`self.FadePPMaterial`))
  (bind _transition (`/Game/Blueprints/GameModes/GI_GameManager.Transition` (`self.Game Instance`)))
  (`GameplayStatics.UnloadStreamLevelBySoftObjectPtr` (`self.Level Normal`))
  (`GameplayStatics.UnloadStreamLevelBySoftObjectPtr` (`self.Level Time Speed`))
  (`GameplayStatics.UnloadStreamLevelBySoftObjectPtr` (`self.Level Time Travel`))
  (`GameplayStatics.UnloadStreamLevelBySoftObjectPtr` (`self.Level Color 1`))
  (`GameplayStatics.UnloadStreamLevelBySoftObjectPtr` (`self.Level Color 2`))
  (`GameplayStatics.UnloadStreamLevelBySoftObjectPtr` (`self.Level Color 3`))
  (`GameplayStatics.UnloadStreamLevelBySoftObjectPtr` (`self.Level Color 4`))
  (`GameplayStatics.UnloadStreamLevelBySoftObjectPtr` (`self.Level Uncanny`))
  (`GameplayStatics.UnloadStreamLevelBySoftObjectPtr` (`self.Level Abnormal`))
  (bind _output_get (set `self.Level Normal` `Level Normal`))
  (bind _output_get_2 (set `self.Level Time Speed` `Level Time Speed`))
  (bind _output_get_3 (set `self.Level Time Travel` `Level Time Travel`))
  (bind _output_get_4 (set `self.Level Color 1` `Level Color 1`))
  (bind _output_get_5 (set `self.Level Color 2` `Level Color 2`))
  (bind _output_get_6 (set `self.Level Color 3` `Level Color 3`))
  (bind _output_get_7 (set `self.Level Color 4` `Level Color 4`))
  (bind _output_get_8 (set `self.Level Uncanny` `Level Uncanny`))
  (bind _output_get_9 (set `self.Level Abnormal` `Level Abnormal`))
  (set `self.Current Level Suffix` "_Normal")
  (set `self.Level Name Prefix` `Level Name Prefix`)
  (`GameplayStatics.LoadStreamLevelBySoftObjectPtr` _output_get true)
  (`GameplayStatics.LoadStreamLevelBySoftObjectPtr` _output_get_2)
  (`GameplayStatics.LoadStreamLevelBySoftObjectPtr` _output_get_3)
  (`GameplayStatics.LoadStreamLevelBySoftObjectPtr` _output_get_4)
  (`GameplayStatics.LoadStreamLevelBySoftObjectPtr` _output_get_5)
  (`GameplayStatics.LoadStreamLevelBySoftObjectPtr` _output_get_6)
  (`GameplayStatics.LoadStreamLevelBySoftObjectPtr` _output_get_7)
  (`GameplayStatics.LoadStreamLevelBySoftObjectPtr` _output_get_8)
  (`GameplayStatics.LoadStreamLevelBySoftObjectPtr` _output_get_9)
  (bind _asbp_player_rig (cast `/Game/Blueprints/Player/Rig/BP_PlayerRig` (`GameplayStatics.GetPlayerPawn` 0)))
  (bind _capsulecollider (`/Game/Blueprints/Player/Rig/BP_PlayerRig.CapsuleCollider` _asbp_player_rig))
  (`PrimitiveComponent.SetConstraintMode` _capsulecollider "None")
  (`PrimitiveComponent.SetConstraintMode` (`/Game/Blueprints/Player/Rig/BP_PlayerRig.Slippy` _asbp_player_rig) "None")
  (`SceneComponent.K2_SetWorldLocation` _capsulecollider (.location `Player Spawn`) false true)
  (`SceneComponent.K2_SetWorldLocation` (`/Game/Blueprints/Player/Rig/BP_PlayerRig.Slippy` _asbp_player_rig) (.location `Player Spawn`) false true)
  (`SceneComponent.K2_SetWorldRotation` _capsulecollider (.rotation `Player Spawn`) false false)
  (`SceneComponent.K2_SetWorldRotation` (`/Game/Blueprints/Player/Rig/BP_PlayerRig.Slippy` _asbp_player_rig) (.rotation `Player Spawn`) false false)
  (`PrimitiveComponent.SetConstraintMode` _capsulecollider "SixDOF")
  (`PrimitiveComponent.SetConstraintMode` (`/Game/Blueprints/Player/Rig/BP_PlayerRig.Slippy` _asbp_player_rig) "SixDOF")
  (`PrimitiveComponent.SetPhysicsLinearVelocity` _capsulecollider (0.0 0.0 0.0) false "None")
  (`PrimitiveComponent.SetPhysicsLinearVelocity` (`/Game/Blueprints/Player/Rig/BP_PlayerRig.Slippy` _asbp_player_rig) (0.0 0.0 0.0) false "None")
  (`self.Time Dilation Sound Trigger` 1.0 true)
  (bind (_direction _fade _colorfilterunblend) (`Timeline|FadeOutFilter` :!via `PlayFromStart`)
    (:`Update`
      (`MaterialInstanceDynamic.SetScalarParameterValue` _fadeppmaterial "Fade" _fade)
      (`MaterialInstanceDynamic.SetScalarParameterValue` _fadeppmaterial "IsNotFilter" _colorfilterunblend)
      (`/Engine/EditorBlueprintResources/StandardMacros.IsValid` _transition
        (:`Is Valid`
          (`AudioComponent.SetVolumeMultiplier` _transition _fade))))))

(event `Load Anomaly of Type`
  (params (`Anomaly Type` :type "/Game/Blueprints/Anomalies/EAnomalyTypeEnum Enum" :default "NewEnumerator0"))
  (bind _returnvalue (select `/Game/Blueprints/Anomalies/EAnomalyTypeEnum` `Anomaly Type` :`NewEnumerator0` "_Normal" :`NewEnumerator1` "_TimeSpeed" :`NewEnumerator2` "_TimeTravel" :`NewEnumerator3` "_Color1" :`NewEnumerator7` "_Color2" :`NewEnumerator8` "_Color3" :`NewEnumerator9` "_Color4" :`NewEnumerator4` "_Uncanny" :`NewEnumerator5` "_Abnormal" :`NewEnumerator6` "_Normal"))
  (bind _level_name_prefix (`self.Level Name Prefix`))
  (set `LevelStreaming.bShouldBeVisible` true (`GameplayStatics.GetStreamingLevel` (`KismetStringLibrary.Conv_StringToName` (`KismetStringLibrary.Concat_StrStr` _level_name_prefix _returnvalue))))
  (set `LevelStreaming.bShouldBeVisible` false (`GameplayStatics.GetStreamingLevel` (`KismetStringLibrary.Conv_StringToName` (`KismetStringLibrary.Concat_StrStr` _level_name_prefix (`self.Current Level Suffix`)))))
  (set `self.Current Level Suffix` _returnvalue))

(event `self.ReceiveBeginPlay`
  (bind _returnvalue (`GameplayStatics.GetActorOfClass` "/Script/Engine.PostProcessVolume"))
  (`/Engine/EditorBlueprintResources/StandardMacros.IsValid` _returnvalue
    (:`Is Valid`
      (set `self.PPV` _returnvalue)
      (bind _asgi_game_manager (cast `/Game/Blueprints/GameModes/GI_GameManager` (`GameplayStatics.GetGameInstance`))
        (:`then`
          (`/Engine/EditorBlueprintResources/StandardMacros.IsValid` _asgi_game_manager
            (:`Is Valid`
              (bind _output_get (set `self.Game Instance` _asgi_game_manager))
              (bind _fademat (`/Game/Blueprints/GameModes/GI_GameManager.FadeMat` _output_get))
              (set `self.FadePPMaterial` _fademat)
              (bind _output_get_2 (set `self.FadePPBlendable` (make `WeightedBlendables` (`|MakeArray` (make `WeightedBlendable` 1.0 _fademat)))))
              (setmembers `PostProcessSettings` :`StructRef` (`PostProcessVolume.Settings` (`self.PPV`)) :`WeightedBlendables` _output_get_2)
              (bind _returnvalue_2 (`|CreateWidget` "/Game/Widgets/W_PauseMenu.W_PauseMenu_C" (`GameplayStatics.GetPlayerController` 0) :!label _label))
              (bind _output_get_3 (set `self.PausedWidget` _returnvalue_2))
              (`UserWidget.AddToViewport` _output_get_3 1)
              (`Widget.SetVisibility` _output_get_3 "Hidden"))))
        (:`CastFailed`
          (`KismetSystemLibrary.PrintString` "OOF"))))
    (:`Is Not Valid`
      (goto _label))))

(event `Effect Enter Anomaly`
  (params (`Time Dilation` :type "Float (double-precision)"))
  (`self.OnAnomalySwap`)
  (`self.Time Dilation Sound Trigger` `Time Dilation`)
  (bind (_direction _out) (`Timeline|Chroma` :!via `PlayFromStart`)
    (:`Update`
      (setmembers `PostProcessSettings` :`StructRef` (`PostProcessVolume.Settings` (`self.PPV`)) :`SceneFringeIntensity` (* _out 20.0) :`AutoExposureBias` (* _out 2.0)))))

(event `Time Dilation Sound Trigger`
  (params (`Time Dilation` :type "Float (double-precision)") (IsRestart :type Boolean))
  (bind _returnvalue (`GameplayStatics.GetGlobalTimeDilation`))
  (bind _old_time_dilation (`self.Old Time Dilation`))
  (set `self.Old Time Dilation` _returnvalue)
  (if IsRestart
    (set `self.Old Time Dilation` (`AudioComponent.PitchMultiplier` (`/Game/Blueprints/GameModes/GI_GameManager.Music` (`self.Game Instance`)))))
  (`GameplayStatics.SetGlobalTimeDilation` `Time Dilation`)
  (bind _asbp_player_rig (cast `/Game/Blueprints/Player/Rig/BP_PlayerRig` (`GameplayStatics.GetPlayerPawn` 0)))
  (set `Actor.CustomTimeDilation` (/ 1.0 `Time Dilation`) _asbp_player_rig)
  (if (> _old_time_dilation _returnvalue)
    (`|ExecutionSequence`
      (:`then_0`
        (bind (_direction _value) (`Timeline|Timeline_1` :!via `Stop` :!label _label_2)
          (:`Update`
            (`self.Set Music Time Dilation` (`KismetMathLibrary.Lerp` _old_time_dilation `Time Dilation` _value)))))
      (:`then_1`
        (bind (_direction_2 _value_2) (`Timeline|Timeline_2` :!via `SetNewTime` :!label _label_3)
          (:`Update`
            (`self.Set Music Time Dilation` (`KismetMathLibrary.Lerp` _old_time_dilation `Time Dilation` _value_2)))))
      (:`then_2`
        (goto _label_3)))
    (elif (< _old_time_dilation _returnvalue)
      (`|ExecutionSequence`
        (:`then_0`
          (goto _label_3 :!via `Stop`))
        (:`then_1`
          (goto _label_2 :!via `SetNewTime`))
        (:`then_2`
          (goto _label_2))))))

(event `Add Rift Maker`
  (set `self.AmountOfRiftMakers` (+ (`self.AmountOfRiftMakers`) 1)))

(event `Remove Rift Maker`
  (set `self.AmountOfRiftMakers` (- (`self.AmountOfRiftMakers`) 1)))

(event `Restart Level`
  (bind _fadeppmaterial (`self.FadePPMaterial`))
  (bind _transition (`/Game/Blueprints/GameModes/GI_GameManager.Transition` (`self.Game Instance`)))
  (if (not (`self.IsDed`))
    (set `self.IsDed` true)
    (`MaterialInstanceDynamic.SetVectorParameterValue` _fadeppmaterial "CurrentFilterColor" (select `int` (`KismetStringLibrary.Conv_StringToInt` (`KismetStringLibrary.Right` (`self.Current Level Suffix`) 1)) :`0` (struct :`R` 1.0 :`G` 1.0 :`B` 1.0 :`A` 1.0) :`1` (struct :`R` 1.0 :`G` 0.088542 :`B` 0.088542 :`A` 1.0) :`2` (struct :`R` 0.306098 :`G` 0.947917 :`B` 0.306098 :`A` 1.0) :`3` (struct :`R` 0.182292 :`G` 0.182292 :`B` 1.0 :`A` 1.0) :`4` (struct :`R` 1.0 :`G` 0.5 :`A` 1.0) :!type "LinearColor Structure"))
    (bind (_direction _fade) (`Timeline|Timeline` :!via `PlayFromStart`)
      (:`Update`
        (`MaterialInstanceDynamic.SetScalarParameterValue` _fadeppmaterial "Fade" _fade)
        (`MaterialInstanceDynamic.SetScalarParameterValue` _fadeppmaterial "IsNotFilter" 0.0)
        (`/Engine/EditorBlueprintResources/StandardMacros.IsValid` _transition
          (:`Is Valid`
            (`AudioComponent.SetVolumeMultiplier` _transition _fade))))
      (:`Finished`
        (`/Game/Blueprints/GameModes/GI_GameManager.Load Level` (`self.Game Instance`) (`KismetStringLibrary.Conv_StringToName` (`self.Level Name Prefix`)))))))

(event `Next Level`
  (bind _fadeppmaterial (`self.FadePPMaterial`))
  (bind _game_instance (`self.Game Instance`))
  (bind _transition (`/Game/Blueprints/GameModes/GI_GameManager.Transition` (`self.Game Instance`)))
  (if (not (`self.IsDed`))
    (set `self.IsDed` true)
    (if (>= (`/Game/Blueprints/GameModes/GI_GameManager.CurrentLevelIndex` _game_instance) (`KismetArrayLibrary.Array_Length` (`/Game/Blueprints/GameModes/GI_GameManager.GameLevels` _game_instance)))
      (`self.Time Dilation Sound Trigger` 1.0 true))
    (`MaterialInstanceDynamic.SetVectorParameterValue` _fadeppmaterial "CurrentFilterColor" (select `int` (`KismetStringLibrary.Conv_StringToInt` (`KismetStringLibrary.Right` (`self.Current Level Suffix`) 1)) :`0` (struct :`R` 1.0 :`G` 1.0 :`B` 1.0 :`A` 1.0) :`1` (struct :`R` 1.0 :`G` 0.088542 :`B` 0.088542 :`A` 1.0) :`2` (struct :`R` 0.306098 :`G` 0.947917 :`B` 0.306098 :`A` 1.0) :`3` (struct :`R` 0.182292 :`G` 0.182292 :`B` 1.0 :`A` 1.0) :`4` (struct :`R` 1.0 :`G` 0.5 :`A` 1.0) :!type "LinearColor Structure"))
    (bind (_direction _fade) (`Timeline|Timeline_0` :!via `PlayFromStart`)
      (:`Update`
        (`MaterialInstanceDynamic.SetScalarParameterValue` _fadeppmaterial "Fade" _fade)
        (`MaterialInstanceDynamic.SetScalarParameterValue` _fadeppmaterial "IsNotFilter" 0.0)
        (`/Engine/EditorBlueprintResources/StandardMacros.IsValid` _transition
          (:`Is Valid`
            (`AudioComponent.SetVolumeMultiplier` _transition _fade))))
      (:`Finished`
        (`/Game/Blueprints/GameModes/GI_GameManager.Next Level` (`self.Game Instance`))))))

(event `Set Music Time Dilation`
  (params (Speed :type "Float (double-precision)"))
  (`AudioComponent.SetPitchMultiplier` (`/Game/Blueprints/GameModes/GI_GameManager.Music` (`self.Game Instance`)) Speed))

(event `Toggle Pause`
  (bind _returnvalue (`GameplayStatics.GetPlayerController` 0))
  (bind _pausedwidget (`self.PausedWidget`))
  (bind _game_instance (`self.Game Instance`))
  (bind _output_get (set `self.IsPaused` (and (not (`self.IsPaused`)) (not (`self.IsDed`)))))
  (bind _returnvalue_2 (`GameplayStatics.SetGamePaused` _output_get))
  (if _output_get
    (`WidgetSwitcher.SetActiveWidgetIndex` (`/Game/Widgets/W_PauseMenu.MenuSwitcher` _pausedwidget) 0)
    (`Widget.SetVisibility` _pausedwidget "Visible")
    (`WidgetBlueprintLibrary.SetInputMode_GameAndUIEx` _returnvalue null "DoNotLock" false)
    (set `PlayerController.bShowMouseCursor` true _returnvalue)
    (`/Game/Blueprints/GameModes/GI_GameManager.Pause Speedrun Timer` _game_instance)
    (`Widget.SetFocus` (`/Game/Widgets/W_PauseMenu.Button_Resume` (`self.PausedWidget`)))
    (else
      (`Widget.SetVisibility` _pausedwidget "Hidden")
      (`WidgetBlueprintLibrary.SetInputMode_GameOnly` (`GameplayStatics.GetPlayerController` 0))
      (`GameplayStatics.SetViewportMouseCaptureMode` "CapturePermanently")
      (set `PlayerController.bShowMouseCursor` false _returnvalue)
      (`/Game/Blueprints/GameModes/GI_GameManager.Run Speedrun Timer` _game_instance))))

(fn `UserConstructionScript`)