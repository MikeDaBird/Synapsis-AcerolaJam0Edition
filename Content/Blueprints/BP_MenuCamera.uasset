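; Main menu camera actor that snaps to the player start, creates the menu widget and sways gently toward the mouse position.
; BeginPlay installs the GameInstance's fade material on the level's post-process volume.
; Timelines drive that material, widget fade and transition audio volume on entry and before level loads.
; Further timelines animate the widget's intro, menu swaps and character bobbing, with the intro gated by a GameInstance flag.
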(event `self.ReceiveBeginPlay`
  (bind _fadeppmaterial (`self.FadePPMaterial`))
  (bind _returnvalue (pcsubsystem `EnhancedInputLocalPlayerSubsystem` (`GameplayStatics.GetPlayerController` 0)))
  (bind _transition (`/Game/Blueprints/GameModes/GI_GameManager.Transition` (`self.Game Instance`)))
  (`/Engine/EditorBlueprintResources/StandardMacros.IsValid` _returnvalue
    (:`Is Valid`
      (`EnhancedInputSubsystemInterface.AddMappingContext` _returnvalue "/Game/Inputs/IMC_Player.IMC_Player" 0 (struct))
      (bind _returnvalue_2 (`GameplayStatics.GetActorOfClass` "/Game/Blueprints/Player/Rig/BP_PlayerStart.BP_PlayerStart_C"))
      (`/Engine/EditorBlueprintResources/StandardMacros.IsValid` _returnvalue_2
        (:`Is Valid`
          (bind _defaultsceneroot (`/Game/Blueprints/Player/Rig/BP_PlayerStart.DefaultSceneRoot` _returnvalue_2))
          (bind _returnvalue_3 (`SceneComponent.K2_GetComponentRotation` _defaultsceneroot))
          (`self.K2_SetActorLocationAndRotation` (`SceneComponent.K2_GetComponentLocation` _defaultsceneroot) _returnvalue_3 false true)
          (set `self.InitialRot` _returnvalue_3)
          (bind _returnvalue_4 (`|CreateWidget` "/Game/Widgets/W_MainMenu.W_MainMenu_C"))
          (bind _output_get (set `self.MenuWidget` _returnvalue_4))
          (`UserWidget.AddToViewport` _output_get 0)
          (bind _returnvalue_5 (`GameplayStatics.GetActorOfClass` "/Script/Engine.PostProcessVolume"))
          (`/Engine/EditorBlueprintResources/StandardMacros.IsValid` _returnvalue_5
            (:`Is Valid`
              (set `self.PPV` _returnvalue_5)
              (bind _asgi_game_manager (cast `/Game/Blueprints/GameModes/GI_GameManager` (`GameplayStatics.GetGameInstance`))
                (:`then`
                  (`/Engine/EditorBlueprintResources/StandardMacros.IsValid` _asgi_game_manager
                    (:`Is Valid`
                      (bind _output_get_2 (set `self.Game Instance` _asgi_game_manager))
                      (bind _fademat (`/Game/Blueprints/GameModes/GI_GameManager.FadeMat` _output_get_2))
                      (set `self.FadePPMaterial` _fademat)
                      (bind _output_get_3 (set `self.FadePPBlendable` (make `WeightedBlendables` (`|MakeArray` (make `WeightedBlendable` 1.0 _fademat)))))
                      (setmembers `PostProcessSettings` :`StructRef` (`PostProcessVolume.Settings` (`self.PPV`)) :`WeightedBlendables` _output_get_3)
                      (if (`/Game/Blueprints/GameModes/GI_GameManager.IntroSequenceRan` (`self.Game Instance`))
                        (bind (_direction _fade _colorfilterunblend) (`Timeline|Timeline` :!label _label)
                          (:`Update`
                            (`MaterialInstanceDynamic.SetScalarParameterValue` _fadeppmaterial "Fade" _fade)
                            (`MaterialInstanceDynamic.SetScalarParameterValue` _fadeppmaterial "IsNotFilter" _colorfilterunblend)
                            (`/Game/Widgets/W_MainMenu.Fade` (`self.MenuWidget`) _fade)
                            (`/Engine/EditorBlueprintResources/StandardMacros.IsValid` _transition
                              (:`Is Valid`
                                (`AudioComponent.SetVolumeMultiplier` _transition (/ _fade 2.0))))))
                        (else
                          (`|ExecutionSequence`
                            (:`then_0`
                              (`self.Init Intro`)
                              (`KismetSystemLibrary.Delay` 1.0)
                              (`self.Intro Anim` false))
                            (:`then_1`
                              (goto _label))))))))
                (:`CastFailed`
                  (`KismetSystemLibrary.PrintString` "OOF"))))))))))

(event `Load Level`
  (params (Name :type Name))
  (bind _fadeppmaterial (`self.FadePPMaterial`))
  (bind _game_instance (`self.Game Instance`))
  (bind _transition (`/Game/Blueprints/GameModes/GI_GameManager.Transition` _game_instance))
  (`|ExecutionSequence`
    (:`then_0`
      (goto _label :!via `Stop`))
    (:`then_1`
      (bind (_direction _fade) (`Timeline|Timeline_0`)
        (:`Update`
          (`MaterialInstanceDynamic.SetScalarParameterValue` _fadeppmaterial "Fade" _fade)
          (`MaterialInstanceDynamic.SetScalarParameterValue` _fadeppmaterial "IsNotFilter" 0.0)
          (`/Game/Widgets/W_MainMenu.Fade` (`self.MenuWidget`) _fade)
          (`/Engine/EditorBlueprintResources/StandardMacros.IsValid` _transition
            (:`Is Valid`
              (`AudioComponent.SetVolumeMultiplier` _transition (/ _fade 2.0)))))
        (:`Finished`
          (`/Game/Blueprints/GameModes/GI_GameManager.Load Level` _game_instance Name))))))

(event `self.ReceiveTick`
  (params (DeltaSeconds :type "Float (single-precision)"))
  (bind _returnvalue (/ (`WidgetLayoutLibrary.GetViewportSize`) 2.0))
  (bind _returnvalue_2 (`WidgetLayoutLibrary.GetMousePositionOnViewport`))
  (bind (_returnvalue_x _returnvalue_y) (`KismetMathLibrary.BreakVector2D` (/ (- (* _returnvalue_2 (`WidgetLayoutLibrary.GetViewportScale`)) _returnvalue) _returnvalue)))
  (set `self.TargetRot` (`KismetMathLibrary.RLerp` (`self.TargetRot`) (`KismetMathLibrary.MakeRotator` 0.0 (`KismetMathLibrary.FClamp` (* _returnvalue_y -1.0) -1.0) (`KismetMathLibrary.FClamp` _returnvalue_x -1.0)) (* DeltaSeconds 3.0) true))
  (`SceneComponent.K2_SetWorldRotation` (`self.Camera`) (`self.InitialRot`) false true)
  (`SceneComponent.K2_AddWorldRotation` (`self.Camera`) (`self.TargetRot`) false false))

(event `Intro Anim`
  (params (`Skip Intro` :type Boolean))
  (bind _menuwidget (`self.MenuWidget`))
  (bind _maincanvas (`/Game/Widgets/W_MainMenu.MainCanvas` (`self.MenuWidget`)))
  (bind _titlebaranim (`/Game/Widgets/W_MainMenu.TitleBarAnim` _menuwidget))
  (bind _mainmenubuttonsanim (`/Game/Widgets/W_MainMenu.MainMenuButtonsAnim` _menuwidget))
  (if `Skip Intro`
    (set `self.IntroTime` 1.85)
    (bind (_direction _title_y _title_opacity _buttons_x _buttons_opacity _copyright_opacity) (`Timeline|Intro Sequence` :`NewTime` (`self.IntroTime`) :!via `SetNewTime` :!label _label_2)
      (:`Update`
        (`Widget.SetRenderTranslation` _titlebaranim (`KismetMathLibrary.MakeVector2D` 0.0 _title_y))
        (`Widget.SetRenderOpacity` _titlebaranim _title_opacity)
        (`Widget.SetRenderTranslation` _mainmenubuttonsanim (`KismetMathLibrary.MakeVector2D` _buttons_x))
        (`Widget.SetRenderOpacity` _mainmenubuttonsanim _buttons_opacity)
        (`Widget.SetRenderOpacity` (`/Game/Widgets/W_MainMenu.MainMenuCopyrightAnim` _menuwidget) _copyright_opacity)
        (`Widget.SetRenderOpacity` (`/Game/Widgets/W_MainMenu.Button_Quit` _menuwidget) _copyright_opacity))
      (:`Enable Input`
        (`Widget.SetVisibility` _maincanvas "Visible")
        (set `/Game/Blueprints/GameModes/GI_GameManager.IntroSequenceRan` true (`self.Game Instance`))
        (`Widget.SetFocus` (`/Game/Widgets/W_MainMenu.Button_NewGame` (`self.MenuWidget`)))))
    (else
      (`Widget.SetVisibility` _maincanvas "HitTestInvisible")
      (goto _label_2))))

(event `Init Intro`
  (bind _menuwidget (`self.MenuWidget`))
  (set `self.IntroTime` 0.0)
  (`Widget.SetFocus` (`/Game/Widgets/W_MainMenu.UnfocusButton` _menuwidget))
  (`Widget.SetVisibility` (`/Game/Widgets/W_MainMenu.MainCanvas` _menuwidget) "HitTestInvisible")
  (goto _label_2 :!via `SetNewTime`))

(event `Swap Menu Animation`
  (bind _transitionanim (`/Game/Widgets/W_MainMenu.TransitionAnim` (`self.MenuWidget`)))
  (bind (_direction _x_translation _opacity) (`Timeline|Transition Animation` :!via `PlayFromStart`)
    (:`Update`
      (`Widget.SetRenderTranslation` _transitionanim (`KismetMathLibrary.MakeVector2D` _x_translation))
      (`Widget.SetRenderOpacity` _transitionanim _opacity))))

(event `Start Bobbing Anim for Char`
  (bind (_direction _newtrack_0) (`Timeline|Character Bob Animation`)
    (:`Update`
      (`Widget.SetRenderTranslation` (`/Game/Widgets/W_MainMenu.CharacterPreview` (`self.MenuWidget`)) (`KismetMathLibrary.MakeVector2D` -28.0 (+ (* _newtrack_0 5.0) 36.0))))))

(fn `UserConstructionScript`)